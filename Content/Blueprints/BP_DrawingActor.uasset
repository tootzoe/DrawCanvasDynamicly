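; Actor that provides a 2D paint surface, viewed through its own orthographic camera in unlit mode.
; On BeginPlay it creates a BP_DrawingCanvas, feeds its dynamic texture into the plane's material, and sizes plane and camera to the canvas.
; Touch press and move deproject screen positions to canvas pixels and draw a dot or decal there.
; Right mouse button cycles between two decal brushes and the dot brush.
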(event EventBeginPlay
  (Development|ExecuteConsoleCommand "viewmode unlit" 0)
  (Game|Player|SetViewTargetwithBlend (Game|GetPlayerController 0) self 0.0 "VTBlend_Linear" 0.0 false)
  (CallFunction|InitializeDrawingCanvas))

(event Input|MouseEvents|RightMouseButton
  (params (Key :type Key%20Structure :default "None"))
  (bind _canvas (Variables|Default|GetCanvas))
  (:Pressed
    (bind _result (Math|Integer|IncrementInt (Variables|Default|GetBrushToolsIdx))
      (:%20%20
        (bind _output_get (Variables|Default|SetBrushToolsIdx (Math|Integer|%(Integer) _result 3)))
        (switch int _output_get
          (:Default
            (Variables|Default|SetIsUseDecal false))
          (:0
            (Class|DrawingCanvas|InitializeDecal _canvas "/Game/Textures/pingvinTexture.pingvinTexture")
            (Variables|Default|SetIsUseDecal true :!label _label))
          (:1
            (Class|DrawingCanvas|InitializeDecal _canvas "/Game/Icons/Android_15_icon.Android_15_icon")
            (goto _label)))))))

(event Input|TouchEvents|InputTouch
  (params (Location :type Vector) (FingerIndex :type ETouchIndex%20Enum))
  (bind _returnvalue (Game|GetPlayerController 0))
  (bind _canvas (Variables|Default|GetCanvas))
  (bind _canvaswidth (Variables|Default|GetCanvasWidth))
  (bind _canvasheight (Variables|Default|GetCanvasHeight))
  (bind _worldlocation (Class|PlayerController|DeprojectScreenPositiontoWorld _returnvalue (.x Location) (.y Location)))
  (bind _returnvalue_2 (/ _canvasheight 2))
  (bind _returnvalue_3 (/ _canvaswidth 2))
  (bind _returnvalue_4 (+ (.y _worldlocation) _returnvalue_2))
  (bind _returnvalue_5 (+ (.x _worldlocation) _returnvalue_3))
  (bind _returnvalue_6 (Math|Float|Round _returnvalue_4))
  (bind _returnvalue_7 (Math|Float|Round _returnvalue_5))
  (:Pressed
    (if (or (!= (Variables|Default|GetMousePosX) _returnvalue_7) (!= _returnvalue_6 (Variables|Default|GetCanvasHeight))) :!label _label
      (if (Variables|Default|GetIsUseDecal)
        (Class|DrawingCanvas|DrawDecal _canvas _returnvalue_7 _returnvalue_6)
        (else
          (Class|DrawingCanvas|DrawDot _canvas _returnvalue_7 _returnvalue_6)))))
  (:Released
    (Variables|Default|SetMousePosX -1)
    (Variables|Default|SetMousePosY -1))
  (:Moved
    (goto _label)))

(fn ConstructionScript)

(fn InitializeDrawingCanvas
  (Variables|/Script/Engine.PlayerController|SetbShowMouseCursor (Game|GetPlayerController 0) true)
  (bind _returnvalue (Game|ConstructObjectfromClass "/Game/Blueprints/BP_DrawingCanvas.BP_DrawingCanvas_C"))
  (bind _output_get (Variables|Default|SetCanvas _returnvalue))
  (Class|DrawingCanvas|InitializeCanvas _output_get (Variables|Default|GetCanvasWidth) (Variables|Default|GetCanvasHeight))
  (Class|DrawingCanvas|InitializeDrawingTools (Variables|Default|GetCanvas) 10)
  (bind _returnvalue_2 (Rendering|Material|CreateDynamicMaterialInstance (Variables|Default|GetCanvasPlane) 0 "/Game/Materials/M_CanvasMaterial.M_CanvasMaterial" "None" :!class /Script/Engine.PrimitiveComponent))
  (bind _output_get_2 (Variables|Default|SetCanvasMaterial _returnvalue_2))
  (Rendering|Material|SetTextureParameterValue _output_get_2 "TexInput" (Variables|/Script/DrawCanvasDynamicly.DrawingCanvas|GetDynamicCanvas (Variables|Default|GetCanvas)))
  (Class|DrawingCanvas|InitializeDecal (Variables|Default|GetCanvas) "/Game/Icons/Android_15_icon.Android_15_icon")
  (Transformation|SetRelativeScale3D (Variables|Default|GetCanvasPlane) (Math|Vector|MakeVector (Math|Conversions|ToFloat(Integer) (/ (Variables|Default|GetCanvasWidth) 100)) (Math|Conversions|ToFloat(Integer) (/ (Variables|Default|GetCanvasHeight) 100)) 1.0))
  (Class|CameraComponent|SetOrthoWidth (Variables|Default|GetCamera) (Math|Conversions|ToFloat(Integer) (Variables|Default|GetCanvasWidth))))